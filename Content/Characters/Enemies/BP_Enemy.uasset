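; BP_Enemy is an enemy pawn that moves toward a target and awards the player money when it dies.
; MoveToTarget uses AIMoveTo and, on failure, calls itself again after a short delay without passing the target.
; On ability system activation, it binds to RootHealthAttributeSet changes, treating any new value at or below zero as death.
; Death adds a truncated attribute value to PlayerStatsSubsystem money, then destroys the actor.
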(event `MoveToTarget`
  (params (TargetActor :type "Actor Object Reference"))
  (`|AIMoveTo` self (0.0 0.0 0.0) TargetActor
    (:`OnFail`
      (`KismetSystemLibrary.Delay` 1.0)
      (`self.MoveToTarget` null))))

(event `self.AbilitySystemComponent.OnComponentActivated`
  (params (Component :type "ActorComponent Object Reference") (bReset :type Boolean))
  (bind _returnvalue (`AbilitySystemComponent.GetAttributeSet` (`self.AbilitySystemComponent`) "/Script/GGJ23.RootHealthAttributeSet"))
  (bind _asroot_health_attribute_set (cast `RootHealthAttributeSet` _returnvalue))
  (add `RootAttributeSetBase.OnPostAttributeChange` _asroot_health_attribute_set (delegate `Health Changed`)))

(event `Health Changed`
  (params (AttributeSet :type "RootAttributeSetBase Object Reference") (Attribute :type "GameplayAttribute Structure (by ref)") (NewValue :type "Float (single-precision)") (OldValue :type "Float (single-precision)"))
  ;[1 1 1] Check Health Value on Modify
  (if (<= NewValue 0.0)
    (`self.OnDeath`)))

(event `OnDeath`
  (bind (_bfound _returnvalue) (`AbilitySystemComponent.GetGameplayAttributeValue` (`self.AbilitySystemComponent`) (struct :`AttributeName` "Money" :`Attribute` "/Script/GGJ23.RootMoneyAttributeSet:Money" :`AttributeOwner` "/Script/CoreUObject.Class'\"/Script/GGJ23.RootMoneyAttributeSet\"'")))
  (`|ExecutionSequence`
    (:`then_0`
      (if _bfound
        (`PlayerStatsSubsystem.AddMoney` (subsystem `PlayerStatsSubsystem`) (`KismetMathLibrary.FTrunc` _returnvalue))))
    (:`then_1`
      (`self.K2_DestroyActor`))))

(fn `UserConstructionScript`
  (`parent.UserConstructionScript`))