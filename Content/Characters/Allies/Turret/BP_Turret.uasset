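; Allied turret that automatically targets nearby enemies and fires pellets at them.
; Sphere overlaps maintain a list of actors tagged Enemy, locking onto the first and retargeting when the current one leaves.
; Tick smoothly yaws toward the target, while a looping reload timer, plus each new lock, triggers the Attack.ShootPellet gameplay ability.
; GetProjectileSpawnTransform supplies a transform at the spawn point aimed directly at the target.
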(event `self.ReceiveTick`
  (params (DeltaSeconds :type "Float (single-precision)"))
  ;[1 0.9807 0.3265] EventTick
  (`/Engine/EditorBlueprintResources/StandardMacros.IsValid` (`self.CurrentTargettedEnemy`)
    (:`Is Valid`
      (`self.LookAtTarget`))))

(event `self.ReceiveBeginPlay`
  (bind _reloadtime (`self.ReloadTime`))
  ;[1 1 1] AttemptToSpawnPellet
  (`KismetSystemLibrary.K2_SetTimerDelegate` (delegate `AttemptToSpawnPellet`) _reloadtime true _reloadtime))

(event `LookAtTarget`
  ;[1 0.884 0.2825] LookAtTarget
  (`self.K2_SetActorRotation` (`KismetMathLibrary.RLerp` (`self.K2_GetActorRotation`) (`KismetMathLibrary.MakeRotator` 0.0 0.0 (.yaw (`KismetMathLibrary.FindLookAtRotation` (`self.K2_GetActorLocation` self) (`self.K2_GetActorLocation` (`self.CurrentTargettedEnemy`))))) 0.1)))

(event `AttemptToSpawnPellet`
  ;[1 1 1] AttemptToSpawnPellet
  (`/Engine/EditorBlueprintResources/StandardMacros.IsValid` (`self.CurrentTargettedEnemy`)
    (:`Is Valid`
      (`self.SpawnBP_Pellet`))))

(event `SpawnBP_Pellet`
  ;[1 0.9883 0.2711] SpawnPellet
  (`AbilitySystemComponent.TryActivateAbilitiesByTag` (`self.AbilitySystemComponent`) (`BlueprintGameplayTagLibrary.MakeGameplayTagContainerFromTag` (struct :`TagName` "Attack.ShootPellet")) true))

(event `self.TurretSphereCollision.OnComponentBeginOverlap`
  (params (OverlappedComponent :type "PrimitiveComponent Object Reference") (OtherActor :type "Actor Object Reference") (OtherComp :type "PrimitiveComponent Object Reference") (OtherBodyIndex :type Integer) (bFromSweep :type Boolean) (SweepResult :type "HitResult Structure (by ref)"))
  ;[0.1729 1 0.3234] BeginOverlap
  (if (!= self OtherActor)
    (bind _tagcontainer (message `GameplayTagAssetInterface.GetOwnedGameplayTags` OtherActor))
    (if (`BlueprintGameplayTagLibrary.HasTag` _tagcontainer (struct :`TagName` "Enemy"))
      (`self.AddTargettableEnemy` OtherActor))))

(event `AddTargettableEnemy`
  (params (Enemy :type "Actor Object Reference (by ref)"))
  ;[1 0.7839 0.2481] AddTargettableEnemy
  (`KismetArrayLibrary.Array_AddUnique` (`self.TargettableEnemies`) Enemy)
  (`self.UpdateTarget`))

(event `UpdateTarget`
  ;[0.5208 1 1] UpdateTarget
  (`/Engine/EditorBlueprintResources/StandardMacros.IsValid` (`self.CurrentTargettedEnemy`)
    (:`Is Not Valid`
      (if (not (`KismetArrayLibrary.Array_IsEmpty` (`self.TargettableEnemies`)))
        (`self.SetTarget` (`|GetArrayItem` (`self.TargettableEnemies`)))))))

(event `SetTarget`
  (params (ActorToTarget :type "Actor Object Reference"))
  ;[0.9905 1 0.2118] SetTarget
  (set `self.CurrentTargettedEnemy` ActorToTarget)
  (`self.AttemptToSpawnPellet`))

(event `self.TurretSphereCollision.OnComponentEndOverlap`
  (params (OverlappedComponent :type "PrimitiveComponent Object Reference") (OtherActor :type "Actor Object Reference") (OtherComp :type "PrimitiveComponent Object Reference") (OtherBodyIndex :type Integer))
  ;[1 0.3953 0.5054] EndOverlap
  (`self.RemoveTargettableEnemy` OtherActor))

(event `RemoveTargettableEnemy`
  (params (ActorToRemove :type "Actor Object Reference (by ref)"))
  ;[1 0.4262 0.4561] RemoveTargettableEnemy
  (`KismetArrayLibrary.Array_RemoveItem` (`self.TargettableEnemies`) ActorToRemove)
  (if (== ActorToRemove (`self.CurrentTargettedEnemy`))
    (set `self.CurrentTargettedEnemy` null)
    (`self.UpdateTarget`)))

(fn `GetProjectileSpawnTransform`
  (returns (SpawnTransform :type "Transform Structure"))
  (bind _returnvalue (`SceneComponent.K2_GetComponentLocation` (`self.ProjectileSpawnPoint`)))
  (return (`KismetMathLibrary.MakeTransform` _returnvalue (`KismetMathLibrary.FindLookAtRotation` _returnvalue (`self.K2_GetActorLocation` (`self.CurrentTargettedEnemy`))))))

(fn `UserConstructionScript`
  (`parent.UserConstructionScript`))