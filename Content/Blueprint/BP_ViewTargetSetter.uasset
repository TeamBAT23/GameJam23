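; BP_ViewTargetSetter is a trigger actor that switches the player's camera while their pawn is inside its box.
; On overlap begin, the pawn's PlayerController blends its view to the ViewTarget variable over BlendTime.
; On overlap end, it blends back to the pawn over the same time.
; Actors that are not pawns controlled by a PlayerController are ignored.
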(event `self.Box.OnComponentBeginOverlap`
  (params (OverlappedComponent :type "PrimitiveComponent Object Reference") (OtherActor :type "Actor Object Reference") (OtherComp :type "PrimitiveComponent Object Reference") (OtherBodyIndex :type Integer) (bFromSweep :type Boolean) (SweepResult :type "HitResult Structure (by ref)"))
  (bind _aspawn (cast `Pawn` OtherActor))
  (bind _asplayer_controller (cast `PlayerController` (`Pawn.GetController` _aspawn)))
  (`PlayerController.SetViewTargetWithBlend` _asplayer_controller (`self.ViewTarget`) (`self.Blend Time`) "VTBlend_Linear" 0.0 false))

(event `self.Box.OnComponentEndOverlap`
  (params (OverlappedComponent :type "PrimitiveComponent Object Reference") (OtherActor :type "Actor Object Reference") (OtherComp :type "PrimitiveComponent Object Reference") (OtherBodyIndex :type Integer))
  (bind _aspawn (cast `Pawn` OtherActor))
  (bind _asplayer_controller (cast `PlayerController` (`Pawn.GetController` _aspawn)))
  (`PlayerController.SetViewTargetWithBlend` _asplayer_controller _aspawn (`self.Blend Time`) "VTBlend_Linear" 0.0 false))

(fn `UserConstructionScript`)