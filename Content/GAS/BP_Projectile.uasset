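; BP_Projectile is a GAS projectile that delivers a gameplay effect to overlapped enemies, optionally homing on a target actor.
; On BeginPlay it homes on ActorToHome's root component if that actor is valid.
; On overlap it ignores its instigator, requires an Enemy tag, and applies the EffectHandle container spec once per actor, tracked in HitActors.
; An enemy overlap also destroys the projectile when DestroyOnCollision is set.
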(event `self.ReceiveBeginPlay`
  (bind _actortohome (`self.ActorToHome`))
  (bind _projectilemovement (`self.ProjectileMovement`))
  (`/Engine/EditorBlueprintResources/StandardMacros.IsValid` _actortohome
    (:`Is Valid`
      (set `ProjectileMovementComponent.bIsHomingProjectile` true _projectilemovement)
      (set `ProjectileMovementComponent.HomingTargetComponent` (`Actor.RootComponent` _actortohome) _projectilemovement))))

(event `self.ReceiveActorBeginOverlap`
  (params (OtherActor :type "Actor Object Reference"))
  ;[1 0.9074 0.3476] Handle projectile overlap
  ;;[0.6692 0.4647 1] Check we aren't self colliding
  (if (!= (`self.GetInstigator`) OtherActor)
    (bind _tagcontainer (message `GameplayTagAssetInterface.GetOwnedGameplayTags` OtherActor))
    (if (`BlueprintGameplayTagLibrary.HasTag` _tagcontainer (struct :`TagName` "Enemy"))
      (`|ExecutionSequence`
        (:`then_0`
          ;;[0.6692 0.4647 1] Check we have't hit before
          (if (not (`KismetArrayLibrary.Array_Contains` (`self.Hit Actors`) OtherActor))
            ;;[0.0786 0.6707 1] Prevent re-entry
            (`KismetArrayLibrary.Array_Add` (`self.Hit Actors`) OtherActor)
            ;;[0.4104 0.4825 1] Apply spec to any targets specified in the effect plus the hit actor
            (bind _returnvalue (`RootAbilitiesUtility.AddTargetsToTargetedEffect` :`InContainerSpec` (`self.EffectHandle`) :`TargetActors` (`|MakeArray` OtherActor)))
            (`RootAbilitiesUtility.ApplyTargetedEffect` _returnvalue)))
        (:`then_1`
          (if (`self.Destroy on Collision`)
            (`self.K2_DestroyActor`)))))))

(fn `UserConstructionScript`)